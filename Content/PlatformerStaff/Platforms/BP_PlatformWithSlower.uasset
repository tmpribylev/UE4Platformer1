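; BP_PlatformWithSlower is a platform that places a slower child actor, judging by its names, at a random spot on itself.
; The construction script runs the parent's, then calls SpawnSlower.
; SpawnSlower adds a child actor component at a random point in the Area box, using its relative location and extent, so placement re-rolls whenever construction reruns.
; The event graph holds only disabled default events.
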(fn `SpawnSlower`
  (bind _area (`self.Area`))
  (`AddComponent|NODE_AddChildActorComponent-0` :`RelativeTransform` (`KismetMathLibrary.Conv_VectorToTransform` (`KismetMathLibrary.RandomPointInBoundingBox` (`SceneComponent.RelativeLocation` _area) (`BoxComponent.BoxExtent` _area)))))

(fn `UserConstructionScript`
  (`parent.UserConstructionScript`)
  (`self.SpawnSlower`))