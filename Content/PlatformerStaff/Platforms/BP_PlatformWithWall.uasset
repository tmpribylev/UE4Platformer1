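; BP_PlatformWithWall is a platform Blueprint that places a wall at one of three candidate positions.
; Its construction script runs the parent's, then gathers the relative transforms of three WallPoint components into an array.
; SpawnWall adds a child actor component at a randomly chosen transform from that array, so the position is re-rolled whenever construction runs.
; The event graph holds only disabled default events.
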(fn `SetWallPoints`
  (set `self.WallsPointsArray` (`|MakeArray` (`SceneComponent.GetRelativeTransform` (`self.WallPoint1`)) (`SceneComponent.GetRelativeTransform` (`self.WallPoint2`)) (`SceneComponent.GetRelativeTransform` (`self.WallPoint3`)))))

(fn `SpawnWall`
  (bind _wallspointsarray (`self.WallsPointsArray`))
  (`AddComponent|NODE_AddChildActorComponent-0` :`RelativeTransform` (`|GetArrayItem` _wallspointsarray (`KismetMathLibrary.RandomIntegerInRange` 0 (`KismetArrayLibrary.Array_LastIndex` _wallspointsarray)))))

(fn `UserConstructionScript`
  (`parent.UserConstructionScript`)
  (`self.SetWallPoints`)
  (`self.SpawnWall`))