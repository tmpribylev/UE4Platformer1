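; BP_GeneralPlatform is a floor tile for a platformer, spawned in sequence through the game mode.
; When the player character overlaps EndTrigger, it asks PlatformerGameMode to add a floor tile, enables gravity on Floor, and destroys itself two seconds later.
; Overlapping DeadZone calls Death on the character.
; GetAttachPoint returns the AttachPoint world transform.
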(event `self.EndTrigger.OnComponentBeginOverlap`
  (params (OverlappedComponent :type "PrimitiveComponent Object Reference") (OtherActor :type "Actor Object Reference") (OtherComp :type "PrimitiveComponent Object Reference") (OtherBodyIndex :type Integer) (bFromSweep :type Boolean) (SweepResult :type "HitResult Structure (by ref)"))
  (cast `/Game/PlatformerStaff/PlatformPersonBP/Blueprints/PlatformPersonCharacter` OtherActor)
  (bind _asplatformer_game_mode (cast `/Game/PlatformerStaff/PlatformPersonBP/Blueprints/PlatformerGameMode` (`GameplayStatics.GetGameMode`)))
  (`/Game/PlatformerStaff/PlatformPersonBP/Blueprints/PlatformerGameMode.AddFloorTile` _asplatformer_game_mode)
  (`PrimitiveComponent.SetEnableGravity` (`self.Floor`) true)
  (`KismetSystemLibrary.Delay` 2.0)
  (`self.K2_DestroyActor`))

(event `self.DeadZone.OnComponentBeginOverlap`
  (params (OverlappedComponent :type "PrimitiveComponent Object Reference") (OtherActor :type "Actor Object Reference") (OtherComp :type "PrimitiveComponent Object Reference") (OtherBodyIndex :type Integer) (bFromSweep :type Boolean) (SweepResult :type "HitResult Structure (by ref)"))
  (bind _asplatform_person_character (cast `/Game/PlatformerStaff/PlatformPersonBP/Blueprints/PlatformPersonCharacter` OtherActor))
  (`/Game/PlatformerStaff/PlatformPersonBP/Blueprints/PlatformPersonCharacter.Death` _asplatform_person_character))

(fn `GetAttachPoint`
  (returns (AttachPoint :type "Transform Structure"))
  (return (`SceneComponent.K2_GetComponentToWorld` (`self.AttachPoint`))))

(fn `UserConstructionScript`)