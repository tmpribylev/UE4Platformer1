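; Enemy actor for a platform that roams between random target points and calls Death on the player character when its sphere is hit.
; It takes the arrow array from its parent BP_PlatformWithEnemy and picks a new random arrow whenever it nears the current one.
; Each tick it smoothly turns toward the target and steps forward by a per-frame speed, reduced while the player's IsSlower flag is set.
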(event `self.Sphere.OnComponentHit`
  (params (HitComponent :type "PrimitiveComponent Object Reference") (OtherActor :type "Actor Object Reference") (OtherComp :type "PrimitiveComponent Object Reference") (NormalImpulse :type "Vector Structure") (Hit :type "HitResult Structure (by ref)"))
  ;[1 1 1] PlayerDeath
  (bind _asplatform_person_character (cast `/Game/PlatformerStaff/PlatformPersonBP/Blueprints/PlatformPersonCharacter` OtherActor))
  (`/Game/PlatformerStaff/PlatformPersonBP/Blueprints/PlatformPersonCharacter.Death` _asplatform_person_character))

(event `self.ReceiveBeginPlay`
  ;[1 1 1] Init and Choose first target
  (`self.InitTargetArray`)
  (set `self.CurrentTP` (`self.GetRandomTargetPoint`))
  (bind _asplatform_person_character (cast `/Game/PlatformerStaff/PlatformPersonBP/Blueprints/PlatformPersonCharacter` (`GameplayStatics.GetPlayerCharacter` 0)))
  (set `self.PlayerRef` _asplatform_person_character))

(event `self.ReceiveTick`
  (params (DeltaSeconds :type "Float (single-precision)"))
  ;[1 1 1] Move
  (`self.K2_SetActorLocationAndRotation` (`self.GetNextLocation`) (`self.GetNextRotation`))
  (if (<= (`self.GetDistanceToComponent` (`self.CurrentTP`)) 75.0)
    (set `self.CurrentTP` (`self.GetRandomTargetPoint`))))

(fn `InitTargetArray`
  (bind _asbp_platform_with_enemy (cast `/Game/PlatformerStaff/Platforms/BP_PlatformWithEnemy` (`self.GetParentActor`)))
  (set `self.ArrowArray` (`/Game/PlatformerStaff/Platforms/BP_PlatformWithEnemy.ArrowArray` _asbp_platform_with_enemy)))

(fn `UserConstructionScript`)