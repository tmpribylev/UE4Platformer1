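; BP_PlatformWithCoins is a platform Blueprint that scatters a random number of coins within its CoinArea box.
; The construction script runs the parent's script, then calls SpawnCoins, which adds up to ten child actor components at random points inside the box.
; Because placement happens at construction, the layout rerolls whenever that script reruns.
; The event graph holds only disabled default nodes, so this Blueprint adds no runtime event logic.
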(fn `SpawnCoins`
  (bind _coinarea (`self.CoinArea`))
  (for _ (range (+ (`KismetMathLibrary.RandomIntegerInRange` 0 10) 1))
    (`AddComponent|NODE_AddChildActorComponent-0` :`RelativeTransform` (`KismetMathLibrary.Conv_VectorToTransform` (`KismetMathLibrary.RandomPointInBoundingBox` (`SceneComponent.RelativeLocation` _coinarea) (`BoxComponent.BoxExtent` _coinarea))))))

(fn `UserConstructionScript`
  (`parent.UserConstructionScript`)
  (`self.SpawnCoins`))