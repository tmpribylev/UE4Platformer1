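; Platform Blueprint that builds enemy spawn content in its construction script via SpawnEnemy.
; SpawnEnemy adds a batch of arrow components into ArrowArray plus one child actor component, all placed through GetRandomLocationVector.
; That helper holds MovementArea random-point nodes, but they are unused.
; InitTargetArray is empty, TargetPoint spawning and tag-filter logic is disconnected, and the event graph adds no behavior.
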(event `self.ReceiveBeginPlay`
  (`parent.ReceiveBeginPlay`))

(fn `InitTargetArray`)

(fn `SpawnEnemy`
  (for _ (range 11)
    (bind _returnvalue (`AddComponent|NODE_AddArrowComponent-0` :`RelativeTransform` (`KismetMathLibrary.Conv_VectorToTransform` (`self.GetRandomLocationVector`))))
    (`KismetArrayLibrary.Array_Add` (`self.ArrowArray`) _returnvalue))
  (`AddComponent|NODE_AddChildActorComponent-0` :`RelativeTransform` (`KismetMathLibrary.Conv_VectorToTransform` (`self.GetRandomLocationVector`)))
  (`self.InitTargetArray`))

(fn `UserConstructionScript`
  (`parent.UserConstructionScript`)
  (`self.SpawnEnemy`))